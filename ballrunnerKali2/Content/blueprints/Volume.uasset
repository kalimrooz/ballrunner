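; Level-exit volume Blueprint meant to advance the game through a list of level names once no Diax actors remain.
; The overlap check for the player and remaining Diax actors is disconnected, so the Box overlap currently does nothing.
; Completelevel quits on the final level or opens the next name in Lvlnames.
; The current-index lookup always returns 0, leaving its name search unused.
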(event `self.Box.OnComponentBeginOverlap`
  (params (OverlappedComponent :type "PrimitiveComponent Object Reference") (OtherActor :type "Actor Object Reference") (OtherComp :type "PrimitiveComponent Object Reference") (OtherBodyIndex :type Integer) (bFromSweep :type Boolean) (SweepResult :type "HitResult Structure (by ref)")))

(fn `completelevel`
  (if (`self.isfinallvl`)
    (`KismetSystemLibrary.QuitGame` null "Quit")
    (else
      (`self.loadnxtlvl`))))

(fn `Getcurrentlvlindex`
  (returns (NewParam :type Integer))
  (bind _returnvalue (`GameplayStatics.GetCurrentLevelName` true))
  (return 0))

(fn `getnxtlvlname`
  (returns (NewParam :type Name))
  (return (`|GetArrayItem` (`self.lvlnames`) (+ (`self.Getcurrentlvlindex`) 1))))

(fn `isfinallvl`
  (returns (returnvalue :type Boolean))
  (return (== (`KismetArrayLibrary.Array_LastIndex` (`self.lvlnames`)) (`self.Getcurrentlvlindex`))))

(fn `loadnxtlvl`
  (`GameplayStatics.OpenLevel` (`self.getnxtlvlname`)))

(fn `UserConstructionScript`)